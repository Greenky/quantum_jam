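; BP_shield is a shield sphere actor that adapts its mesh to whether the local player camera is inside it.
; Each Tick it measures the distance from player 0's camera to the sphere center against a fixed radius.
; ClientInside and ClientOutside swap between the normal and inverted-normals sphere meshes, using an IsInside flag so the mesh changes only on crossing.
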(event Custom|ClientInside
  (if (not (Variables|Default|GetisInside))
    (Components|StaticMesh|SetStaticMesh (Variables|Default|GetSphere) "/Engine/EditorMeshes/AssetViewer/Sphere_inversenormals.Sphere_inversenormals")
    (Variables|Default|SetisInside true)))

(event Custom|ClientOutside
  (if (Variables|Default|GetisInside)
    (Components|StaticMesh|SetStaticMesh (Variables|Default|GetSphere) "/Engine/BasicShapes/Sphere.Sphere")
    (Variables|Default|SetisInside false)))

(event EventBeginPlay)

(event Collision|EventActorBeginOverlap
  (params (OtherActor :type Actor%20Object%20Reference)))

(event EventTick
  (params (DeltaSeconds :type Float%20%28single-precision%29))
  (if (< (Math|Vector|Distance(Vector) (Camera|GetCameraLocation (Game|GetPlayerCameraManager 0)) (Transformation|GetWorldLocation (Variables|Default|GetSphere))) 3e+02)
    (CallFunction|ClientInside)
    (else
      (CallFunction|ClientOutside))))

(fn ConstructionScript)