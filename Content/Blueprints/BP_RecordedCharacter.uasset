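; Character that replays a player's recorded turn from MoveRecorderData save data, with team materials and a mesh per character type.
; Tick steps through timestamped samples, lerping transform, deriving velocity and re-firing recorded shots and skills (mine or shield projectile), then notifies the game mode when finished.
; When downed it becomes a collisionless team-colored hologram that keeps replaying movement without attacking.
; StopReplay rewinds to the first sample and clears the ghost state.
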(event OnDowned(HealthComponent)
  ;[0.15 0.15 0.15 0.5] On Death
  (CallFunction|ServerCreateGhost))

(event OnHealthChanged(HealthComponent)
  (params (health :type Integer) (healthNormalized :type Float%20%28double-precision%29)))

(event Custom|ClientCreateGhost
  (params (TeamIndex :type Integer))
  ;[0.15 0.15 0.15 0.5] On Death
  (Variables|Default|SetisDead true)
  (Collision|SetActorEnableCollision self false)
  (CallFunction|CreateGhost TeamIndex))

(event Custom|SpawnMine
  (params (Location :type Vector))
  ;[0.15 0.15 0.15 0.5] Skills
  (Game|SpawnActorfromClass "/Game/Blueprints/BP_Mine.BP_Mine_C" (Math|Transform|MakeTransform Location "0, 0, 0" "1.000000,1.000000,1.000000") "Undefined" "MultiplyWithRoot" 0 0))

(event Custom|ClientResetGhost
  (params (TeamIndex :type Integer))
  ;[0.15 0.15 0.15 0.5] Reset Hologram materials
  (Collision|SetActorEnableCollision self true)
  (CallFunction|ResetGhost TeamIndex))

(event Custom|AIUseSkill
  ;[0.15 0.15 0.15 0.5] Skills
  (if (== (Variables|/Game/Blueprints/MoveRecorderData.MoveRecorderData_C|GetcharacterType (Variables|Default|GetMove%20Recorder%20Data)) 1)
    (CallFunction|ShootMine)
    (else
      (CallFunction|ShootShield))))

(event Custom|TestSound
  (params (Location :type Vector))
  (Audio|PlaySoundatLocation "/Game/FirstPerson/FPWeapon/Audio/FirstPersonTemplateWeaponFire02.FirstPersonTemplateWeaponFire02" Location "0, 0, 0" 0.1 1.0 0.0 0 0 0 0) ; Play firing sound
)

(event Custom|ServerResetGhost
  ;[0.15 0.15 0.15 0.5] Reset Hologram materials
  (Variables|Default|SetisDead false)
  (Collision|SetActorEnableCollision self true)
  (CallFunction|ClientResetGhost (Variables|Default|GetTeamIndex)))

(event Custom|ServerCreateGhost
  ;[0.15 0.15 0.15 0.5] On Death
  (Variables|Default|SetisDead true)
  (Collision|SetActorEnableCollision self false)
  (CallFunction|ClientCreateGhost (Variables|Default|GetTeamIndex)))

(event Custom|ShootMine
  (bind _returnvalue (Transformation|GetActorLocation))
  (bind _returnvalue_2 (Class|KismetMathLibrary|VectorForward))
  (bind _camerarotation (Variables|Default|GetcameraRotation))
  (bind _returnvalue_3 (Math|Vector|RotateVector _returnvalue_2 _camerarotation))
  (bind _returnvalue_4 (+ _returnvalue "-10.000000,0.000000,60.000000"))
  (bind _returnvalue_5 (* _returnvalue_3 1e+02))
  (bind _returnvalue_6 (+ _returnvalue_4 _returnvalue_5))
  ;[0.15 0.15 0.15 0.5] Skills
  (Game|SpawnActorfromClass "/Game/Blueprints/BP_MineProjectile.BP_MineProjectile_C" (Math|Transform|MakeTransform _returnvalue_6 _camerarotation "1.000000,1.000000,1.000000") "Undefined" "OverrideRootScale" self 0 2e+03 1 0)
  (CallFunction|TestSound _returnvalue_6))

(event Custom|ServerSetupMaterials
  (params (PlayerIndex :type Integer))
  (bind _tp_body (Variables|Default|GetTP_Body))
  (bind _bp_weapon_component (Variables|Default|GetBP_Weapon_Component))
  (bind _charactertype (Variables|Default|GetCharacterType))
  ;[0.15 0.15 0.15 0.5] Materials for differnt teams
  (Variables|Default|SetTeamIndex PlayerIndex)
  (if (== _charactertype 0)
    (Components|SkeletalMesh|SetSkeletalMeshAsset _bp_weapon_component "/Game/FirstPerson/FPWeapon/Mesh/SKM_Pistol.SKM_Pistol")
    (Default|ResetupWeapon _bp_weapon_component "hand_lSocket")
    (Components|SkeletalMesh|SetSkeletalMeshAsset _tp_body "/Game/Characters/Mannequins/Meshes/SKM_MiniManny.SKM_MiniManny")
    (elif (== _charactertype 1)
      _
      (else
        (Components|SkeletalMesh|SetSkeletalMeshAsset _bp_weapon_component "/Game/FirstPerson/FPWeapon/Mesh/SK_BigGun1.SK_BigGun1")
        (Components|SkeletalMesh|SetSkeletalMeshAsset _tp_body "/Game/Characters/Mannequins/Meshes/SKM_MegaManny.SKM_MegaManny"))))
  (CallFunction|ClientSetupMaterials PlayerIndex _charactertype))

(event Custom|ClientSetupMaterials
  (params (PlayerIndex :type Integer) (CharType :type Integer))
  (bind _tp_body (Variables|Default|GetTP_Body))
  (bind _bp_weapon_component (Variables|Default|GetBP_Weapon_Component))
  (bind _tp_body_2 (Variables|Default|GetTP_Body))
  ;[0.15 0.15 0.15 0.5] Materials for differnt teams
  (Utilities|FlowControl|Sequence
    (:then_0
      (if (== PlayerIndex 0)
        (Rendering|Material|SetMaterial _tp_body 0 "/Game/Materials/MI_TeamA01.MI_TeamA01")
        (Rendering|Material|SetMaterial _tp_body 1 "/Game/Materials/MI_TeamA02.MI_TeamA02")
        (else
          (Rendering|Material|SetMaterial _tp_body 0 "/Game/Materials/MI_TeamB01.MI_TeamB01")
          (Rendering|Material|SetMaterial _tp_body 1 "/Game/Materials/MI_TeamB02.MI_TeamB02"))))
    (:then_1
      (if (== CharType 0)
        (Components|SkeletalMesh|SetSkeletalMeshAsset _bp_weapon_component "/Game/FirstPerson/FPWeapon/Mesh/SKM_Pistol.SKM_Pistol")
        (Default|ResetupWeapon _bp_weapon_component "hand_lSocket")
        (Components|SkeletalMesh|SetSkeletalMeshAsset _tp_body_2 "/Game/Characters/Mannequins/Meshes/SKM_MiniManny.SKM_MiniManny")
        (elif (not (== CharType 1))
          (Components|SkeletalMesh|SetSkeletalMeshAsset _bp_weapon_component "/Game/FirstPerson/FPWeapon/Mesh/SK_BigGun1.SK_BigGun1")
          (Components|SkeletalMesh|SetSkeletalMeshAsset _tp_body_2 "/Game/Characters/Mannequins/Meshes/SKM_MegaManny.SKM_MegaManny"))))))

(event Custom|StartReplay
  (params (CurrentTurnNumber :type Integer))
  (Variables|Default|SetcanReplay true)
  ;[0.15 0.15 0.15 0.5] Update helth bar visibility and health
  (Default|RefillHealth (Variables|Default|GetHealthComponent)))

(event Custom|StopReplay
  (Variables|Default|SetcanReplay false)
  (Transformation|SetRelativeTransform (Variables|/Script/Engine.MovementComponent|GetUpdatedPrimitive (Variables|Character|GetCharacterMovement)) (Utilities|Array|Get(acopy) (Variables|/Game/Blueprints/MoveRecorderData.MoveRecorderData_C|GetTransformData (Variables|Default|GetMove%20Recorder%20Data))) false true)
  (CallFunction|ResetValues)
  (if (Variables|Default|GetisDead)
    (CallFunction|ServerResetGhost)))

(event Custom|SpawnShield
  (params (Location :type Vector))
  ;[0.15 0.15 0.15 0.5] Skills
  (Game|SpawnActorfromClass "/Game/Blueprints/BP_shield.BP_shield_C" (Math|Transform|MakeTransform Location "0, 0, 0" "1.000000,1.000000,1.000000") "Undefined" "MultiplyWithRoot" 0 0))

(event Custom|Setup%20replay
  (params (SlotName :type String) (UserIndex :type Integer) (TurnNumber :type Integer))
  (Variables|Default|SetRecordedTurnNumber TurnNumber)
  (if (Utilities|IsValid (Variables|Default|GetMove%20Recorder%20Data))
    (Variables|Default|SetcanReplay true :!label _label)
    (Variables|Default|SetCurrentTransform (Utilities|Array|Get(acopy) (Variables|/Game/Blueprints/MoveRecorderData.MoveRecorderData_C|GetTransformData (Variables|Default|GetMove%20Recorder%20Data))))
    (Variables|Default|SetOldPosition (.location (Utilities|Array|Get(acopy) (Variables|/Game/Blueprints/MoveRecorderData.MoveRecorderData_C|GetTransformData (Variables|Default|GetMove%20Recorder%20Data)))))
    (Variables|Default|SetCharacterType (Variables|/Game/Blueprints/MoveRecorderData.MoveRecorderData_C|GetcharacterType (Variables|Default|GetMove%20Recorder%20Data)))
    (else
      (bind _returnvalue (SaveGame|LoadGamefromSlot SlotName))
      (bind _asmove_recorder_data (Utilities|Casting|CastToMoveRecorderData _returnvalue)
        (:then
          (Variables|Default|SetMove%20Recorder%20Data _asmove_recorder_data)
          (goto _label))
        (:CastFailed
          (Development|PrintString "Error loading save"))))))

(event Custom|ShootShield
  (bind _returnvalue (Transformation|GetActorLocation))
  (bind _returnvalue_2 (Class|KismetMathLibrary|VectorForward))
  (bind _camerarotation (Variables|Default|GetcameraRotation))
  (bind _returnvalue_3 (Math|Vector|RotateVector _returnvalue_2 _camerarotation))
  (bind _returnvalue_4 (+ _returnvalue "-10.000000,0.000000,60.000000"))
  (bind _returnvalue_5 (* _returnvalue_3 1e+02))
  (bind _returnvalue_6 (+ _returnvalue_4 _returnvalue_5))
  ;[0.15 0.15 0.15 0.5] Skills
  (Game|SpawnActorfromClass "/Game/Blueprints/BP_ShieldProjectile.BP_ShieldProjectile_C" (Math|Transform|MakeTransform _returnvalue_6 _camerarotation "1.000000,1.000000,1.000000") "Undefined" "OverrideRootScale" self 0 2e+03 1 0)
  (CallFunction|TestSound _returnvalue_6))

(event EventTick
  (params (DeltaSeconds :type Float%20%28single-precision%29))
  (bind _healthbar (Variables|Default|GetHealthBar))
  (bind _healthcomponent (Variables|Default|GetHealthComponent))
  (bind _recordingindex (Variables|Default|GetrecordingIndex))
  (bind _move_recorder_data (Variables|Default|GetMove%20Recorder%20Data))
  (bind _move_recorder_data_2 (Variables|Default|GetMove%20Recorder%20Data))
  (bind _recordingindex_2 (Variables|Default|GetrecordingIndex))
  (bind _recordingindex_3 (Variables|Default|GetrecordingIndex))
  (bind _timestamp (Variables|/Game/Blueprints/MoveRecorderData.MoveRecorderData_C|GettimeStamp _move_recorder_data_2))
  (bind _output (Utilities|Array|Get(acopy) _timestamp _recordingindex_3))
  (Utilities|FlowControl|Sequence
    (:then_0
      ;[0.15 0.15 0.15 0.5] Replay Logic with trimestamps
      (if (and (Variables|Default|GetcanReplay) (Utilities|IsValid (Variables|Default|GetMove%20Recorder%20Data)))
        (Variables|Default|SetcurrentTimestamp (+ DeltaSeconds (Variables|Default|GetcurrentTimestamp)))
        (if (>= _output (Variables|Default|GetcurrentTimestamp)) :!label _label
          (Transformation|SetRelativeTransform (Variables|/Script/Engine.MovementComponent|GetUpdatedPrimitive (Variables|Character|GetCharacterMovement)) (Math|Transform|Lerp(Transform) (Variables|Default|GetCurrentTransform) (Utilities|Array|Get(acopy) (Variables|/Game/Blueprints/MoveRecorderData.MoveRecorderData_C|GetTransformData (Variables|Default|GetMove%20Recorder%20Data)) (Variables|Default|GetrecordingIndex)) (Utilities|GetLerpTimeFraction (Variables|Default|GetcurrentTimestamp) (Variables|Default|GetoldTimestamp) _output)) false false)
          (bind _output_get (Variables|Default|SetCurrentTransform (Math|Transform|Lerp(Transform) (Variables|Default|GetCurrentTransform) (Utilities|Array|Get(acopy) (Variables|/Game/Blueprints/MoveRecorderData.MoveRecorderData_C|GetTransformData (Variables|Default|GetMove%20Recorder%20Data)) (Variables|Default|GetrecordingIndex)) (Utilities|GetLerpTimeFraction (Variables|Default|GetcurrentTimestamp) (Variables|Default|GetoldTimestamp) _output))))
          (Variables|Default|SetVelocity (/ (- (.location _output_get) (Variables|Default|GetOldPosition)) DeltaSeconds))
          (Variables|Default|SetOldPosition (.location _output_get))
          (Variables|Default|SetcameraRotation (Utilities|Array|Get(acopy) (Variables|/Game/Blueprints/MoveRecorderData.MoveRecorderData_C|GetCameraRotation _move_recorder_data) _recordingindex_2))
          (Variables|Default|SetoldTimestamp (Variables|Default|GetcurrentTimestamp))
          (Variables|Default|SetinAir (Utilities|Array|Get(acopy) (Variables|/Game/Blueprints/MoveRecorderData.MoveRecorderData_C|GetinAir _move_recorder_data) _recordingindex_2))
          (if (not (Variables|Default|GetisDead))
            (Utilities|FlowControl|Sequence
              (:then_0
                (if (Variables|Default|GetisShooting)
                  (Default|AIWeponShooting (Variables|Default|GetBP_Weapon_Component))))
              (:then_1
                (if (Variables|Default|GetisUsingSkill)
                  (CallFunction|AIUseSkill)))
              (:then_2
                (Variables|Default|SetisShooting false :!label _label_2)
                (Variables|Default|SetisUsingSkill false)))
            (else
              (goto _label_2)))
          (else
            (if (Utilities|Array|Get(acopy) (Variables|/Game/Blueprints/MoveRecorderData.MoveRecorderData_C|GetisShooting _move_recorder_data_2) _recordingindex_3)
              (Variables|Default|SetisShooting true))
            (if (Utilities|Array|Get(acopy) (Variables|/Game/Blueprints/MoveRecorderData.MoveRecorderData_C|GetisUsingSkill _move_recorder_data_2) _recordingindex_3)
              (Variables|Default|SetisUsingSkill true))
            (if (== (- (Utilities|Array|Length (Variables|/Game/Blueprints/MoveRecorderData.MoveRecorderData_C|GettimeStamp (Variables|Default|GetMove%20Recorder%20Data))) 1) _recordingindex)
              (Transformation|SetRelativeTransform (Variables|/Script/Engine.MovementComponent|GetUpdatedPrimitive (Variables|Character|GetCharacterMovement)) (Utilities|Array|Get(acopy) (Variables|/Game/Blueprints/MoveRecorderData.MoveRecorderData_C|GetTransformData (Variables|Default|GetMove%20Recorder%20Data)) (Variables|Default|GetrecordingIndex)) false false)
              (Variables|Default|SetcanReplay false)
              (bind _asbp_first_person_game_mode (Utilities|Casting|CastToBP_FirstPersonGameMode (Game|GetGameMode)))
              (Default|ReplayFinishedNotification _asbp_first_person_game_mode)
              (else
                (Math|Integer|IncrementInt _recordingindex
                  (:%20%20
                    (goto _label)))))))))
    (:then_1
      ;[0.15 0.15 0.15 0.5] Update health bar
      (if (Rendering|IsVisible _healthbar)
        (Transformation|SetWorldRotation _healthbar (Math|Rotator|FindLookatRotation (Transformation|GetWorldLocation _healthbar) (Transformation|GetWorldLocation (Variables|/Script/Engine.PlayerCameraManager|GetTransformComponent (Game|GetPlayerCameraManager 0)))) false false)
        (bind _asremote_health_bar (Utilities|Casting|CastToRemoteHealthBar (UserInterface|GetWidget _healthbar)))
        (Progress|SetPercent (Variables|/Game/Health/UI/RemoteHealthBar.RemoteHealthBar_C|GetHealthBar _asremote_health_bar) (/ (Variables|/Game/Health/HealthComponent.HealthComponent_C|Gethealth _healthcomponent) (Variables|/Game/Health/HealthComponent.HealthComponent_C|GetmaxHealth _healthcomponent)))))))

(fn ConstructionScript)

(fn CreateGhost
  (params (TeamIndex :type Integer))
  (if (== TeamIndex 0)
    (Rendering|Material|SetMaterial (Variables|Default|GetTP_Body) 0 "/Game/Materials/MI_Hologram_TeamA.MI_Hologram_TeamA")
    (Rendering|Material|SetMaterial (Variables|Default|GetTP_Body) 1 "/Game/Materials/MI_Hologram_TeamA.MI_Hologram_TeamA")
    (Rendering|Material|SetMaterial (Variables|Default|GetBP_Weapon_Component) 0 "/Game/Materials/MI_Hologram_TeamA.MI_Hologram_TeamA")
    (else
      (Rendering|Material|SetMaterial (Variables|Default|GetTP_Body) 0 "/Game/Materials/MI_Hologram_TeamB.MI_Hologram_TeamB")
      (Rendering|Material|SetMaterial (Variables|Default|GetTP_Body) 1 "/Game/Materials/MI_Hologram_TeamB.MI_Hologram_TeamB")
      (Rendering|Material|SetMaterial (Variables|Default|GetBP_Weapon_Component) 0 "/Game/Materials/MI_Hologram_TeamB.MI_Hologram_TeamB"))))

(fn ResetGhost
  (params (TeamIndex :type Integer))
  (Variables|Default|SetisDead false)
  (if (== TeamIndex 0)
    (Rendering|Material|SetMaterial (Variables|Default|GetTP_Body) 0 "/Game/Materials/MI_TeamA01.MI_TeamA01")
    (Rendering|Material|SetMaterial (Variables|Default|GetTP_Body) 1 "/Game/Materials/MI_TeamA02.MI_TeamA02")
    (Rendering|Material|SetMaterial (Variables|Default|GetBP_Weapon_Component) 0 "/Game/FirstPerson/FPWeapon/Materials/M_FPGun.M_FPGun")
    (else
      (Rendering|Material|SetMaterial (Variables|Default|GetTP_Body) 0 "/Game/Materials/MI_TeamB01.MI_TeamB01")
      (Rendering|Material|SetMaterial (Variables|Default|GetTP_Body) 1 "/Game/Materials/MI_TeamB02.MI_TeamB02")
      (Rendering|Material|SetMaterial (Variables|Default|GetBP_Weapon_Component) 0 "/Game/FirstPerson/FPWeapon/Materials/M_FPGun.M_FPGun"))))

(fn ResetValues
  (bind _move_recorder_data (Variables|Default|GetMove%20Recorder%20Data))
  (if (Utilities|IsValid _move_recorder_data)
    (Variables|Default|SetCurrentTransform (Utilities|Array|Get(acopy) (Variables|/Game/Blueprints/MoveRecorderData.MoveRecorderData_C|GetTransformData _move_recorder_data))))
  (Variables|Default|SetcurrentTimestamp 0.0)
  (Variables|Default|SetoldTimestamp 0.0)
  (Variables|Default|SetisShooting false)
  (Variables|Default|SetinAir false)
  (Variables|Default|SetVelocity "0, 0, 0")
  (Variables|Default|SetrecordingIndex 0))