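; Top-down observer actor that hands the player over to a first-person character via a timeline camera glide.
; Pressing Q lerps its transform to the stored Character's camera, or the first PlayerStart, then spawns a character if needed, possesses it and destroys the observer.
; A separate ServerLerp event glides the observer to the spawn point supplied by BP_FirstPersonGameMode.
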(event Custom|ServerLerp
  ;[0.15 0.15 0.15 0.5] LerpMotion
  (bind _asbp_first_person_game_mode (Utilities|Casting|CastToBP_FirstPersonGameMode (Game|GetGameMode)))
  (bind _observerstartpoint (Default|GetMyObserverSpawnpoint _asbp_first_person_game_mode))
  (CallFunction|LerpingMotion (Transformation|GetActorTransform self) (Transformation|GetActorTransform _observerstartpoint)))

(event Custom|LerpingMotion
  (params (StartTransform :type Transform) (EndTransform :type Transform))
  ;[0.15 0.15 0.15 0.5] LerpMotion
  (Variables|Default|SetStartTransform StartTransform)
  (Variables|Default|SetEndTransform EndTransform)
  (bind _lerping (Timeline|Timeline_0 Play)
    (:Update
      (Transformation|SetActorTransform self (Math|Transform|Lerp(Transform) (Variables|Default|GetStartTransform) (Variables|Default|GetEndTransform) _lerping)))))

(event Custom|SpawnAndPosessFPS_Character
  (params (PlayerController :type Player%20Controller%20Object%20Reference))
  (if (Utilities|IsValid (Variables|Default|GetCharacter))
    _
    (else
      (bind _outactors (Actor|GetAllActorsOfClass "/Script/Engine.PlayerStart"))
      (bind _returnvalue (Game|SpawnActorfromClass "/Game/FirstPerson/Blueprints/BP_FirstPersonCharacter.BP_FirstPersonCharacter_C" (Transformation|GetActorTransform (Utilities|Array|Get(acopy) _outactors)) "AdjustIfPossibleButAlwaysSpawn" "MultiplyWithRoot" 0 0))
      (Variables|Default|SetCharacter _returnvalue)))
  (Pawn|Possess PlayerController (Variables|Default|GetCharacter))
  (Actor|DestroyActor))

(event EventBeginPlay
  ;[0.15 0.15 0.15 0.5] Lerp To Anchor position
)

(event EventTick
  (params (DeltaSeconds :type Float%20%28single-precision%29)))

(event Input|KeyboardEvents|Q
  (params (Key :type Key%20Structure :default "None"))
  (:Pressed
    (Variables|Default|SetStartTransform (Transformation|GetActorTransform self))
    (bind _outactors (Actor|GetAllActorsOfClass "/Game/FirstPerson/Blueprints/BP_FirstPersonCharacter.BP_FirstPersonCharacter_C"))
    (if (or (not (Utilities|IsValid (Variables|Default|GetCharacter))) (Utilities|Array|IsEmpty _outactors))
      (bind _outactors_2 (Actor|GetAllActorsOfClass "/Script/Engine.PlayerStart"))
      (Variables|Default|SetEndTransform (Transformation|GetWorldTransform (Variables|/Script/Engine.Actor|GetRootComponent (Utilities|Array|Get(acopy) _outactors_2))))
      (bind _lerping (Timeline|Timeline Play)
        (:Update
          (Transformation|SetActorTransform self (Math|Transform|Lerp(Transform) (Variables|Default|GetStartTransform) (Variables|Default|GetEndTransform) _lerping)))
        (:Finished
          (CallFunction|SpawnandPosessFPSCharacter (Game|GetPlayerController 0))))
      (else
        (Variables|Default|SetEndTransform (Transformation|GetWorldTransform (Variables|/Game/FirstPerson/Blueprints/BP_FirstPersonCharacter.BP_FirstPersonCharacter_C|GetFirstPersonCamera (Variables|Default|GetCharacter))))
        (Timeline|Timeline Play)))))

(fn ConstructionScript)