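; BP_Mine is a proximity mine that damages a character on contact and then destroys itself.
; On BeginPlay it binds the Colision overlap and replays a timeline that continually animates the uniform scale of its Radius component.
; Overlaps cast to BP_FirstPersonCharacter or BP_RecordedCharacter, ignoring other actors.
; A match calls ServerApplyDamage, which prints a message, applies fixed damage to that character and destroys the mine.
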(event Custom|SphereOnOverlap
  (params (OverlappedComponent :type Primitive%20Component%20Object%20Reference) (OtherActor :type Actor%20Object%20Reference) (OtherComp :type Primitive%20Component%20Object%20Reference) (OtherBodyIndex :type Integer) (bFromSweep :type Boolean) (SweepResult :type Hit%20Result%20Structure%20%28by%20ref%29))
  (bind _asbp_first_person_character (Utilities|Casting|CastToBP_FirstPersonCharacter OtherActor)
    (:then
      (CallFunction|ServerApplyDamage _asbp_first_person_character))
    (:CastFailed
      (bind _asbp_recorded_character (Utilities|Casting|CastToBP_RecordedCharacter OtherActor))
      (CallFunction|ServerApplyDamage _asbp_recorded_character))))

(event Custom|ServerApplyDamage
  (params (DamagedActor :type Actor%20Object%20Reference))
  (Development|PrintString "EXPLODE")
  (Game|Damage|ApplyDamage DamagedActor 5e+01 0 0)
  (Actor|DestroyActor))

(event EventBeginPlay
  (Collision|BindEventtoOnComponentBeginOverlap (Variables|Default|GetColision) (delegate Custom|SphereOnOverlap))
  (bind _newtrack_0 (Timeline|RadiusAnimation PlayFromStart)
    (:Update
      (Transformation|SetRelativeScale3D (Variables|Default|GetRadius) (Math|Vector|MakeVector _newtrack_0 _newtrack_0 _newtrack_0)))
    (:Finished
      (Timeline|RadiusAnimation PlayFromStart))))

(fn ConstructionScript)